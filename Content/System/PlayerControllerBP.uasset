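; Test player controller that triggers pathfinding and movement requests from debug keys.
; F and V print a colored notice and call TestAllCharacterMoveToTargetPoint for synchronous or asynchronous pathfinding, respectively.
; G sends the controlled FuncTestProjCharacter to the first actor tagged Destination through SplineMoveToLocation on its MRequestMoveComponent, ignoring spline height.
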(event `Key|F`
  (params (Key :type "Key Structure"))
  (:`Pressed`
    (`KismetSystemLibrary.PrintString` "Start Sync PathFinding Request" true true (struct :`R` 1.0 :`G` 0.052581 :`A` 1.0))
    (`self.Test_AllCharacterMoveToTargetPoint` false)))

(event `Key|V`
  (params (Key :type "Key Structure"))
  (:`Pressed`
    (`KismetSystemLibrary.PrintString` "Start Async PathFinding Request" true true (struct :`R` 0.149375 :`G` 1.0 :`A` 1.0))
    (`self.Test_AllCharacterMoveToTargetPoint` true)))

(event `Key|G`
  (params (Key :type "Key Structure"))
  (:`Pressed`
    (bind _asfunc_test_proj_character (cast `FuncTestProjCharacter` (`self.K2_GetPawn`)))
    (bind _outactors (`GameplayStatics.GetAllActorsWithTag` "Destination"))
    (`RequestMoveComponent.K2_SplineMoveToLocation` (`FuncTestProjCharacter.m_RequestMoveComponent` _asfunc_test_proj_character) (`self.K2_GetActorLocation` (`|GetArrayItem` _outactors)) (make `RequestMoveParams` -1.0) true)))

(fn `UserConstructionScript`)